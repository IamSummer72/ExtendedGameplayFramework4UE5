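; Animation modifier that automatically places foot plant notifies in animation sequences, one track per configured foot.
; On apply it removes listed notifies by name, then samples each foot bone's world position at a fixed step to get horizontal speed.
; Separate unplant and plant speed thresholds act as hysteresis, adding a notify when a moving foot slows down.
; Revert deletes the per-foot notify tracks.
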(event `self.OnApply`
  (params (AnimationSequence :type "AnimSequence Object Reference"))
  (`self.ApplyModifier` AnimationSequence))

(event `self.OnRevert`
  (params (AnimationSequence :type "AnimSequence Object Reference"))
  (`self.RevertModifier` AnimationSequence))

(fn `ApplyModifier`
  (params (AnimSequence :type "AnimSequence Object Reference"))
  (for _array_element (`self.NotifiesToRemove`)
    (`AnimationBlueprintLibrary.RemoveAnimationNotifyEventsByName` (`local.AnimSequence`) _array_element))
  (for _array_element_2 (`self.FeetDefinitions`)
    (`self.ProcessFoot` (`local.AnimSequence`) _array_element_2)))

(fn `ProcessFoot`
  (params (AnimSequence :type "AnimSequence Object Reference") (FootDefinition :type "/Game/Main/Blueprint/SFootFXAnimModifier_FootDefinition Structure"))
  (locals (CurrentTime :type "Float (double-precision)") (LastFootPosition :type "Vector Structure") (CurrentFootPosition :type "Vector Structure") (HasFootUnplanted :type Boolean) (CurrentFootSpeed :type "Float (double-precision)"))
  (bind _animposeevaluationoptions (make `AnimPoseEvaluationOptions` "Raw"))
  (bind _footdefinition_bonename (break `/Game/Main/Blueprint/SFootFXAnimModifier_FootDefinition` (`local.FootDefinition`)))
  (bind _footdefinition_bonename_2 (break `/Game/Main/Blueprint/SFootFXAnimModifier_FootDefinition` (`local.FootDefinition`)))
  (bind (_footdefinition_bonename_3 _footdefinition_notifytrackname _footdefinition_notifytype) (break `/Game/Main/Blueprint/SFootFXAnimModifier_FootDefinition` (`local.FootDefinition`)))
  (bind (_footdefinition_bonename_4 _footdefinition_notifytrackname_2) (break `/Game/Main/Blueprint/SFootFXAnimModifier_FootDefinition` (`local.FootDefinition`)))
  (`AnimationBlueprintLibrary.AddAnimationNotifyTrack` (`local.AnimSequence`) _footdefinition_notifytrackname_2)
  (bind _pose (`AnimPoseExtensions.GetAnimPoseAtTime` (`local.AnimSequence`) 0.0 _animposeevaluationoptions))
  (set `local.LastFootPosition` (.location (`AnimPoseExtensions.GetBonePose` _pose _footdefinition_bonename_2 "World")))
  (set `local.HasFootUnplanted` false)
  (for _index (range 1 (+ (`KismetMathLibrary.FTrunc` (/ (`AnimationBlueprintLibrary.GetSequenceLength` (`local.AnimSequence`)) (`self.SampleStep`))) 1))
    (set `local.CurrentTime` (* _index (`self.SampleStep`)))
    (bind _pose_2 (`AnimPoseExtensions.GetAnimPoseAtTime` (`local.AnimSequence`) (`local.CurrentTime`) _animposeevaluationoptions))
    (set `local.CurrentFootPosition` (.location (`AnimPoseExtensions.GetBonePose` _pose_2 _footdefinition_bonename "World")))
    (set `local.CurrentFootSpeed` (/ (`KismetMathLibrary.VSizeXY` (- (`local.CurrentFootPosition`) (`local.LastFootPosition`))) (`self.SampleStep`)))
    (set `local.LastFootPosition` (`local.CurrentFootPosition`))
    (if (`local.HasFootUnplanted`)
      (if (< (`local.CurrentFootSpeed`) (`self.FootPlantedSpeedThreshold`))
        (`AnimationBlueprintLibrary.AddAnimationNotifyEvent` (`local.AnimSequence`) _footdefinition_notifytrackname (`local.CurrentTime`) _footdefinition_notifytype)
        (set `local.HasFootUnplanted` false))
      (elif (> (`local.CurrentFootSpeed`) (`self.FootUnplantedSpeedThreshold`))
        (set `local.HasFootUnplanted` true)))))

(fn `RevertModifier`
  (params (AnimSequence :type "AnimSequence Object Reference"))
  (for _array_element (`self.FeetDefinitions`)
    (`AnimationBlueprintLibrary.RemoveAnimationNotifyTrack` (`local.AnimSequence`) (`.NotifyTrackName_5_E136755641D4EF9847B215952DFEE8C9` (break `/Game/Main/Blueprint/SFootFXAnimModifier_FootDefinition` _array_element)))))