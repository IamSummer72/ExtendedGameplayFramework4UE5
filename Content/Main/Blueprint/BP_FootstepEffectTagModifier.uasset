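; An animation modifier that builds a notify track for footstep effects from the foot plant notifies already in an animation sequence.
; On apply it clears or creates that track, then passes each left or right foot plant's trigger time and foot socket to AddEffectNotifyAndSetParams, whose body is empty here.
; On revert it removes the track.
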(event `self.OnApply`
  (params (AnimationSequence :type "AnimSequence Object Reference"))
  (`self.RemoveExistingNotifies` AnimationSequence)
  (`self.AddNotifyTrack` AnimationSequence)
  (bind _output_get (set `self.Notify Events` (`AnimationBlueprintLibrary.GetAnimationNotifyEvents` AnimationSequence)))
  (for _array_element _output_get
    (bind _returnvalue (`GameplayStatics.GetObjectClass` (`.Notify` (break `AnimNotifyEvent` _array_element))))
    (if (== _returnvalue "/Game/Main/Blueprint/AN_FootPlant_Left.AN_FootPlant_Left_C")
      (bind _returnvalue_2 (`AnimationBlueprintLibrary.GetAnimNotifyEventTriggerTime` _array_element))
      (`self.AddEffectNotifyAndSetParams` AnimationSequence _returnvalue_2 "foot_l")
      (elif (== _returnvalue "/Game/Main/Blueprint/AN_FootPlant_Right.AN_FootPlant_Right_C")
        (`self.AddEffectNotifyAndSetParams` AnimationSequence _returnvalue_2 "foot_r")))))

(event `self.OnRevert`
  (params (AnimationSequence :type "AnimSequence Object Reference"))
  (`AnimationBlueprintLibrary.RemoveAnimationNotifyTrack` AnimationSequence (`self.NotifyTrackName`)))

(fn `AddEffectNotifyAndSetParams`
  (params (AnimSequence :type "AnimSequence Object Reference") (StartTime :type "Float (double-precision)") (SocketName :type Name)))

(fn `AddNotifyTrack`
  (params (AnimSequence :type "AnimSequence Object Reference"))
  (set `self.bHasTrack` false)
  (for _array_element (`AnimationBlueprintLibrary.GetAnimationNotifyTrackNames` AnimSequence)
    (if (== _array_element (`self.NotifyTrackName`))
      (set `self.bHasTrack` true)))
  (if (not (`self.bHasTrack`))
    (`AnimationBlueprintLibrary.AddAnimationNotifyTrack` AnimSequence (`self.NotifyTrackName`) (struct :`G` 0.786888 :`B` 1.0 :`A` 1.0))))

(fn `RemoveExistingNotifies`
  (params (AnimSequence :type "AnimSequence Object Reference"))
  (`AnimationBlueprintLibrary.RemoveAnimationNotifyEventsByTrack` AnimSequence (`self.NotifyTrackName`)))