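; Animation modifier that bakes turn yaw and weight curves into an animation sequence, apparently for turn-in-place animations.
; For each frame, it reads the root bone's local yaw and keys the turn remaining until the final frame's yaw.
; The weight curve holds at 1 until the first frame where remaining yaw is nearly zero, then keys 0 one frame later.
; Reverting removes both curves.
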(event `self.OnApply`
  (params (AnimationSequence :type "AnimSequence Object Reference"))
  (`AnimationBlueprintLibrary.AddCurve` AnimationSequence (`self.TurnYawCurveName`))
  (bind _firstzeroturnyawframe (`self.PopulateCurveKeys` AnimationSequence))
  (`AnimationBlueprintLibrary.AddCurve` AnimationSequence (`self.WeightCurveName`))
  (`AnimationBlueprintLibrary.AddFloatCurveKey` AnimationSequence (`self.WeightCurveName`) 0.0 1.0)
  (`AnimationBlueprintLibrary.AddFloatCurveKey` AnimationSequence (`self.WeightCurveName`) (`AnimationBlueprintLibrary.GetTimeAtFrame` AnimationSequence _firstzeroturnyawframe) 1.0)
  (`AnimationBlueprintLibrary.AddFloatCurveKey` AnimationSequence (`self.WeightCurveName`) (`AnimationBlueprintLibrary.GetTimeAtFrame` AnimationSequence (+ _firstzeroturnyawframe 1))))

(event `self.OnRevert`
  (params (AnimationSequence :type "AnimSequence Object Reference"))
  (`AnimationBlueprintLibrary.RemoveCurve` AnimationSequence (`self.TurnYawCurveName`))
  (`AnimationBlueprintLibrary.RemoveCurve` AnimationSequence (`self.WeightCurveName`)))

(fn `PopulateCurveKeys`
  (params (AnimSequence :type "AnimSequence Object Reference"))
  (returns (FirstZeroTurnYawFrame :type Integer))
  (locals (TotalTurnYaw :type "Float (double-precision)") (NumFrames :type Integer) (FirstZeroTurnFrame :type Integer :default -1))
  (set `local.NumFrames` (`AnimationBlueprintLibrary.GetNumFrames` (`local.AnimSequence`)))
  (bind _pose (`AnimPoseExtensions.GetAnimPoseAtFrame` (`local.AnimSequence`) (`local.NumFrames`)))
  (set `local.TotalTurnYaw` (.yaw (.rotation (`AnimPoseExtensions.GetBonePose` _pose (`self.RootBoneName`)))))
  (for _index (range (+ (`local.NumFrames`) 1))
    (bind _pose_2 (`AnimPoseExtensions.GetAnimPoseAtFrame` (`local.AnimSequence`) _index (make `AnimPoseEvaluationOptions` "Raw")))
    (bind _returnvalue (- (`local.TotalTurnYaw`) (.yaw (.rotation (`AnimPoseExtensions.GetBonePose` _pose_2 (`self.RootBoneName`))))))
    (`AnimationBlueprintLibrary.AddFloatCurveKey` (`local.AnimSequence`) (`self.TurnYawCurveName`) (`AnimationBlueprintLibrary.GetTimeAtFrame` (`local.AnimSequence`) _index) _returnvalue)
    (if (and (`KismetMathLibrary.NearlyEqual_FloatFloat` _returnvalue) (== (`local.FirstZeroTurnFrame`) -1))
      (set `local.FirstZeroTurnFrame` _index)))
  (return (`local.FirstZeroTurnFrame`)))